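; BP_DoorDrawing is a puzzle door that opens when a chosen set of buttons is pressed with no incorrect ones active.
; On BeginPlay it gathers every BP_Button referencing it and builds the combination from a user-set list.
; Combination presses and releases feed the parent door's condition count.
; Other linked buttons adjust an incorrect-input counter, which blocks opening, closes a satisfied door, or retries opening once cleared.
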(event EventOneLessCondition
  (params (Caller :type BP%20Object%20Object%20Reference))
  (bind _m_totalbuttonsreferencing (Variables|Default|GetM%20TotalButtonsReferencing))
  (bind _m_drawingbuttons (Variables|Default|GetM%20DrawingButtons))
  ;[1 1 1] Button pressed back
  (bind _output_get (Variables|Default|SetM%20Caller Caller))
  (if (Utilities|IsButton _output_get)
    ;;[1 1 1 1 25] Is it a button part of the combination ?
    (bind _return (CallFunction|IsPartOfArrayButtons (Variables|Default|GetM%20Caller) _m_drawingbuttons))
    (if (>= _return 0)
      (Utilities|Array|SetArrayElem _m_drawingbuttons _return (Utilities|Struct|MakeSTRUCT_DrawingCaller (.button (Utilities|Array|Get(acopy) _m_drawingbuttons _return)) false))
      (if (>= _return 0) :!label _label
        (|CallParentFunction (Variables|Default|GetM%20Caller))
        (elif (> (Variables|Default|GetM%20IncorrectInputs) 0)
          (bind _result (Math|Integer|DecrementInt (Variables|Default|GetM%20IncorrectInputs))
            (:%20%20
              (CallFunction|TryOpening (and (== _result 0) (== (Variables|Default|GetM%20NbConditions) (Variables|Default|GetM%20VerifiedCondition))))))))
      (else
        ;;[1 1 1 1 25] Is it at least a button part of all the buttons referencing this door ?
        (bind _return_2 (CallFunction|IsPartOfArrayButtons (Variables|Default|GetM%20Caller) _m_totalbuttonsreferencing))
        (if (>= _return_2 0)
          (Utilities|Array|SetArrayElem _m_totalbuttonsreferencing 0 (Utilities|Struct|MakeSTRUCT_DrawingCaller (.button (Utilities|Array|Get(acopy) _m_totalbuttonsreferencing _return_2)) false))
          (goto _label))))))

(event EventOneMoreCondition
  (params (Caller :type BP%20Object%20Object%20Reference) (CanOpen :type Boolean))
  (bind _m_incorrectinputs (Variables|Default|GetM%20IncorrectInputs))
  (bind _m_verifiedcondition (Variables|Default|GetM%20VerifiedCondition))
  (bind _m_nbconditions (Variables|Default|GetM%20NbConditions))
  (bind _m_drawingbuttons (Variables|Default|GetM%20DrawingButtons))
  (bind _m_totalbuttonsreferencing (Variables|Default|GetM%20TotalButtonsReferencing))
  ;[1 1 1] Button pressed
  (bind _output_get (Variables|Default|SetM%20Caller Caller))
  (if (Utilities|IsButton _output_get)
    ;;[1 1 1 1 25] Is it a button part of the combination ?
    (bind _return (CallFunction|IsPartOfArrayButtons (Variables|Default|GetM%20Caller) _m_drawingbuttons))
    (if (>= _return 0)
      (Utilities|Array|SetArrayElem _m_drawingbuttons _return (Utilities|Struct|MakeSTRUCT_DrawingCaller (.button (Utilities|Array|Get(acopy) _m_drawingbuttons _return)) true))
      (if (>= _return 0) :!label _label
        (Development|PrintString (Utilities|String|Append "Incorrects : " (Utilities|String|ToString(Integer) _m_incorrectinputs) "Corrects : " (Utilities|String|ToString(Integer) _m_verifiedcondition) "Total : \\n" (Utilities|String|ToString(Integer) _m_nbconditions)))
        (|CallParentFunction (Variables|Default|GetM%20Caller) (== (stale _result) 0))
        (else
          (bind _result (Math|Integer|IncrementInt _m_incorrectinputs)
            (:%20%20
              (if (and (not (== _result 0)) (== _m_nbconditions _m_verifiedcondition))
                (CallFunction|CloseDoor))))))
      (else
        ;;[1 1 1 1 25] Is it at least a button part of all the buttons referencing this door ?
        (bind _return_2 (CallFunction|IsPartOfArrayButtons (Variables|Default|GetM%20Caller) _m_totalbuttonsreferencing))
        (if (>= _return_2 0)
          (Utilities|Array|SetArrayElem _m_totalbuttonsreferencing 0 (Utilities|Struct|MakeSTRUCT_DrawingCaller (.button (Utilities|Array|Get(acopy) _m_totalbuttonsreferencing _return_2)) true))
          (goto _label))))))

(event EventBeginPlay
  ;[0 1 0.208] Construction of TotalButtonsReferencing
  (bind _outactors (Actor|GetAllActorsOfClass "/Game/Blueprints/Actors/Interactables/BP_Button.BP_Button_C"))
  (for _array_element _outactors
    (bind _door (Default|GetReferencedDoor _array_element))
    (if (== self _door)
      (Utilities|Array|Add (Variables|Default|GetM%20TotalButtonsReferencing) (Utilities|Struct|MakeSTRUCT_DrawingCaller _array_element false))))
  ;[0 1 0.1628] Construction of DrawingButtons
  (for _array_element_2 (Variables|Default|GetM%20DrawingButtonsUser)
    (Utilities|Array|Add (Variables|Default|GetM%20DrawingButtons) (Utilities|Struct|MakeSTRUCT_DrawingCaller _array_element_2 false))))

(fn ConstructionScript
  (|CallParentFunction)
  (Variables|Default|SetM%20IncorrectInputs 0)
  (Variables|Default|SetM%20CurrentButtPartOfCombi false))

(fn IsPartOfArrayButtons
  (params (Button :type BP%20Object%20Object%20Reference) (Array :type Array%20of%20STRUCT%20Drawing%20Caller%20Structures))
  (for (_array_element _array_index) Array
    (if (== (.Button (Utilities|Struct|BreakSTRUCT_DrawingCaller _array_element)) Button)
      (return _array_index)))
  (return -1))
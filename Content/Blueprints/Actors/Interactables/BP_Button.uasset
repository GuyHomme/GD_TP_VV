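; Pressable button interactable that adds or removes an open condition on its referenced door.
; BeingPressed always allows activation, but only releases an already pressed button when MCanSwitch is set.
; Each toggle plays a sound, swaps the button materials and runs a timeline forward or in reverse to spin the mesh and change the light color.
; ResetButton calls ResetObject, then clears the pressed state and restores the inactive material.
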(event Custom|BeingPressed
  (bind _audio (Variables|Default|GetAudio))
  (if (not (Variables|State|GetM%20Pressed))
    (bind _output_get (Variables|State|SetM%20Pressed (not (Variables|State|GetM%20Pressed)) :!label _label))
    (if _output_get
      (Audio|Components|Audio|Play _audio 0.0)
      ;[1 1 1] Button pressed
      (Default|OneMoreCondition (Variables|Components|GetM%20Door) self true)
      (for (_ _array_index) (Rendering|Material|GetMaterials (Variables|Default|GetButton))
        (Rendering|Material|SetMaterial (Variables|Default|GetButton) _array_index (Variables|Components|GetM%20MatActivated)))
      ;[1 1 1] Animations
      (bind (_direction _rotation _lightcolor) (Timeline|M%20Activation Play)
        (:Update
          (Transformation|SetWorldRotation (Variables|Default|GetButton) (Math|Rotator|Lerp(Rotator) "0, 0, 0" (Math|Rotator|MakeRotator 0.0 0.0 3.6e+02) _rotation) false false)
          (Rendering|Components|Light|SetLightColor (Variables|Default|GetLight) _lightcolor true)))
      (else
        (Audio|Components|Audio|Play _audio 0.0)
        ;[1 1 1] Button pressed back
        (Default|OneLessCondition (Variables|Components|GetM%20Door) self)
        (for (_ _array_index_2) (Rendering|Material|GetMaterials (Variables|Default|GetButton))
          (Rendering|Material|SetMaterial (Variables|Default|GetButton) _array_index_2 (Variables|Components|GetM%20MatDesactivated)))
        (Timeline|M%20Activation Reverse)))
    (elif (Variables|Components|GetM%20CanSwitch)
      (goto _label))))

(fn ConstructionScript
  (|CallParentFunction)
  (Variables|State|SetM%20Pressed false)
  (Variables|Components|SetM%20MatActivated "/Game/StarterContent/Materials/M_Basic_Floor.M_Basic_Floor")
  (Variables|Components|SetM%20MatDesactivated "/Game/StarterContent/Materials/M_Metal_Burnished_Steel.M_Metal_Burnished_Steel")
  (Rendering|Material|SetMaterial (Variables|Default|GetButton) 0 (Variables|Components|GetM%20MatDesactivated))
  (Audio|Components|Audio|SetSound (Variables|Default|GetAudio) "/Game/Audio/SoundEffect_OrbPoke_Cue.SoundEffect_OrbPoke_Cue"))

(fn GetReferencedDoor
  (return (Variables|Components|GetM%20Door)))

(fn ResetButton
  (CallFunction|ResetObject)
  (Variables|State|SetM%20Pressed false)
  (Rendering|Material|SetMaterial (Variables|Default|GetButton) 0 (Variables|Components|GetM%20MatDesactivated)))